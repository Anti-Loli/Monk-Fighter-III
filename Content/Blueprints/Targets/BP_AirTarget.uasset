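; BP_AirTarget is a target actor that reports to a manager through its ManagerRef reference.
; When destroyed, it removes the first entry from the manager's PurpleTargets array, regardless of which target was destroyed.
; Its BeginPlay, overlap and Tick events are disabled stubs, and the construction script only calls the parent.
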(event EventBeginPlay
  (|CallParentFunction) ; This node is disabled and will not be called.\nDrag off pins to build functionality.
)

(event Collision|EventActorBeginOverlap
  (params (OtherActor :type Actor%20Object%20Reference))
  (|CallParentFunction OtherActor) ; This node is disabled and will not be called.\nDrag off pins to build functionality.
)

(event EventTick
  (params (DeltaSeconds :type Float%20%28single-precision%29))
  (|CallParentFunction DeltaSeconds) ; This node is disabled and will not be called.\nDrag off pins to build functionality.
)

(event EventDestroyed
  (Utilities|Array|RemoveIndex (Variables|/Game/Blueprints/Tutorial_Managers/Basic/BP_Tutorial_Manager_Basics.BP_Tutorial_Manager_Basics_C|GetPurple%20Targets (Variables|Default|GetManager%20Ref))))

(fn ConstructionScript
  (|CallParentFunction))