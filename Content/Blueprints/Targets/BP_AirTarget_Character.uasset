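; BP_AirTarget_Character is an air target Blueprint that updates a manager's target list when it is destroyed.
; Its Destroyed event removes index 0 from TargetArray on CmanagerRef, so it drops the first entry rather than looking itself up.
; BeginPlay, overlap and Tick are disabled stubs, and the construction script only calls its parent.
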(event EventBeginPlay
  (|CallParentFunction) ; This node is disabled and will not be called.\nDrag off pins to build functionality.
)

(event Collision|EventActorBeginOverlap
  (params (OtherActor :type Actor%20Object%20Reference))
  (|CallParentFunction OtherActor) ; This node is disabled and will not be called.\nDrag off pins to build functionality.
)

(event EventTick
  (params (DeltaSeconds :type Float%20%28single-precision%29))
  (|CallParentFunction DeltaSeconds) ; This node is disabled and will not be called.\nDrag off pins to build functionality.
)

(event EventDestroyed
  (Utilities|Array|RemoveIndex (Variables|/Game/Blueprints/Tutorial_Managers/Character/BP_Character_Tutorial_Manager.BP_Character_Tutorial_Manager_C|GetTarget%20Array (Variables|Default|GetCmanager%20ref))))

(fn ConstructionScript
  (|CallParentFunction))