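; Tutorial manager that judges a target-clearing challenge and reports the result on the WBP_Character widgets.
; Every Tick, it pushes any change in TargetArray's length to those widgets as TargetNum.
; Once the array no longer holds two targets, a one-second Delay starts, after which an empty array shows success text and anything else shows fail text.
; Either result sets Complete, which stops further checks.
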(event EventBeginPlay)

(event Collision|EventActorBeginOverlap
  (params (OtherActor :type Actor%20Object%20Reference)))

(event EventTick
  (params (DeltaSeconds :type Float%20%28single-precision%29))
  (CallFunction|UpdateTargetNum)
  ;[1 1 1] Checks if tutorial has been complete
  (if (not (Variables|Default|Getcomplete))
    ;[1 1 1] Checks if the next target is removed from the array in time
    (if (not (== (Utilities|Array|Length (Variables|Default|GetTarget%20Array)) 2))
      (Utilities|FlowControl|Delay 1.0)
      (if (== (Utilities|Array|Length (Variables|Default|GetTarget%20Array)) 0)
        (Variables|Default|Setcomplete true)
        (bind _foundwidgets (Widget|GetAllWidgetsOfClass "/Game/Blueprints/Tutorial_Managers/Character/WBP_Character.WBP_Character_C" true))
        (for _array_element _foundwidgets
          (Default|SetSuccessText _array_element)
          (Utilities|FlowControl|Delay 5.0))
        (else
          (Variables|Default|Setcomplete true)
          (bind _foundwidgets_2 (Widget|GetAllWidgetsOfClass "/Game/Blueprints/Tutorial_Managers/Character/WBP_Character.WBP_Character_C" true))
          (for _array_element_2 _foundwidgets_2
            (Default|SetFailText _array_element_2)
            (Utilities|FlowControl|Delay 5.0)))))))

(fn ConstructionScript)

(fn UpdateTargetNum
  (bind _target_array (Variables|Default|GetTarget%20Array))
  (bind _returnvalue (Utilities|Array|Length _target_array))
  (if (!= (Variables|Default|GetMax%20Array%20Len) _returnvalue)
    (Variables|Default|SetMax%20Array%20Len _returnvalue)
    (bind _foundwidgets (Widget|GetAllWidgetsOfClass "/Game/Blueprints/Tutorial_Managers/Character/WBP_Character.WBP_Character_C" true))
    (for _array_element _foundwidgets
      (Variables|/Game/Blueprints/Tutorial_Managers/Character/WBP_Character.WBP_Character_C|SetTargetNum _array_element (Variables|Default|GetMax%20Array%20Len)))))