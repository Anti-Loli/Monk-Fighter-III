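; BP_Advanced_Manager judges success or failure in the advanced tutorial based on which targets are destroyed.
; Every Tick it polls reference validity: a lost DestroyTarget means success, while losing either of exactly two NoDestroyTargets means failure.
; Results go to top-level WBP_Advanced1 widgets, found by class, as success or fail text, with success also zeroing TargetNum.
; Nothing latches the result, so searches and updates repeat each frame.
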(event EventBeginPlay)

(event Collision|EventActorBeginOverlap
  (params (OtherActor :type Actor%20Object%20Reference)))

(event EventTick
  (params (DeltaSeconds :type Float%20%28single-precision%29))
  (CallFunction|IsDestroyTarget)
  (CallFunction|IsNoDestroyTarget))

(fn ConstructionScript)

(fn IsDestroyTarget
  ;[1 1 1] Checks if correct target is deystroyed. If it is then tutorial is complete and level ends
  (if (not (Utilities|IsValid (Variables|Default|GetDestroy%20Target)))
    (bind _foundwidgets (Widget|GetAllWidgetsOfClass "/Game/Blueprints/Tutorial_Managers/Advanced/WBP_Advanced1.WBP_Advanced1_C" true))
    (for _array_element _foundwidgets
      (bind _aswbp_advanced_1 (Utilities|Casting|CastToWBP_Advanced1 _array_element))
      (Variables|/Game/Blueprints/Tutorial_Managers/Advanced/WBP_Advanced1.WBP_Advanced1_C|SetTargetNum _aswbp_advanced_1 0)
      (Default|SetSuccessText _aswbp_advanced_1))))

(fn IsNoDestroyTarget
  ;[1 1 1] Checks if one target has been destroyed
  (if (== (Utilities|Array|Length (Variables|Default|GetNo%20destroy%20Targets)) 2)
    ;[1 1 1] Checks if either wrong target in array is destroyed
    (if (not (and (Utilities|IsValid (Utilities|Array|Get(acopy) (Variables|Default|GetNo%20destroy%20Targets))) (Utilities|IsValid (Utilities|Array|Get(acopy) (Variables|Default|GetNo%20destroy%20Targets) 1))))
      ;[1 1 1] If a wrong is deystroyed tutorial fails
      (bind _foundwidgets (Widget|GetAllWidgetsOfClass "/Game/Blueprints/Tutorial_Managers/Advanced/WBP_Advanced1.WBP_Advanced1_C" true))
      (for _array_element _foundwidgets
        (bind _aswbp_advanced_1 (Utilities|Casting|CastToWBP_Advanced1 _array_element))
        (Default|SetFailText _aswbp_advanced_1)))))