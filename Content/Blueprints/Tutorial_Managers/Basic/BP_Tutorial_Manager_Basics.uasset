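; Tutorial manager for the basics tutorial that tracks the remaining green, purple and white targets.
; BeginPlay caches each target array's length, and Tick polls for changes, pushing new counts to top-level WBP_Basic widgets found by class lookup.
; While all three counts are zero, every Tick also calls SetTutorialTextVisibility on those widgets.
; Target removal from the arrays happens outside this graph.
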(event EventBeginPlay
  (Variables|Default|SetGreen%20Array%20Len (Utilities|Array|Length (Variables|Default|GetGreen%20Targets)))
  (Variables|Default|SetPurple%20Array%20Len (Utilities|Array|Length (Variables|Default|GetPurple%20Targets)))
  (Variables|Default|SetWhite%20Array%20Len (Utilities|Array|Length (Variables|Default|GetWhite%20Targets))))

(event Collision|EventActorBeginOverlap
  (params (OtherActor :type Actor%20Object%20Reference)))

(event EventTick
  (params (DeltaSeconds :type Float%20%28single-precision%29))
  (CallFunction|UpdateGreenTargets)
  (CallFunction|UpdateWhiteTargets)
  (CallFunction|UpdatePurpleTargets)
  (CallFunction|AllTargetsDestroyed))

(fn ConstructionScript)

(fn UpdateGreenTargets
  (bind _green_targets (Variables|Default|GetGreen%20Targets))
  (bind _returnvalue (Utilities|Array|Length _green_targets))
  (if (!= (Variables|Default|GetGreen%20Array%20Len) _returnvalue)
    (Variables|Default|SetGreen%20Array%20Len _returnvalue)
    (bind _foundwidgets (Widget|GetAllWidgetsOfClass "/Game/Blueprints/Tutorial_Managers/Basic/WBP_Basic.WBP_Basic_C" true))
    (for _array_element _foundwidgets
      (bind _aswbp_basic (Utilities|Casting|CastToWBP_Basic _array_element))
      (Variables|/Game/Blueprints/Tutorial_Managers/Basic/WBP_Basic.WBP_Basic_C|SetGreen%20Target%20Num _aswbp_basic (Variables|Default|GetGreen%20Array%20Len)))))

(fn UpdateWhiteTargets
  (bind _white_targets (Variables|Default|GetWhite%20Targets))
  (bind _returnvalue (Utilities|Array|Length _white_targets))
  (if (!= (Variables|Default|GetWhite%20Array%20Len) _returnvalue)
    (Variables|Default|SetWhite%20Array%20Len _returnvalue)
    (bind _foundwidgets (Widget|GetAllWidgetsOfClass "/Game/Blueprints/Tutorial_Managers/Basic/WBP_Basic.WBP_Basic_C" true))
    (for _array_element _foundwidgets
      (bind _aswbp_basic (Utilities|Casting|CastToWBP_Basic _array_element))
      (Variables|/Game/Blueprints/Tutorial_Managers/Basic/WBP_Basic.WBP_Basic_C|SetWhite%20Target%20Num _aswbp_basic (Variables|Default|GetWhite%20Array%20Len)))))

(fn UpdatePurpleTargets
  (bind _purple_targets (Variables|Default|GetPurple%20Targets))
  (bind _returnvalue (Utilities|Array|Length _purple_targets))
  (if (!= (Variables|Default|GetPurple%20Array%20Len) _returnvalue)
    (Variables|Default|SetPurple%20Array%20Len _returnvalue)
    (bind _foundwidgets (Widget|GetAllWidgetsOfClass "/Game/Blueprints/Tutorial_Managers/Basic/WBP_Basic.WBP_Basic_C" true))
    (for _array_element _foundwidgets
      (bind _aswbp_basic (Utilities|Casting|CastToWBP_Basic _array_element))
      (Variables|/Game/Blueprints/Tutorial_Managers/Basic/WBP_Basic.WBP_Basic_C|SetPurple%20Target%20Num _aswbp_basic (Variables|Default|GetPurple%20Array%20Len)))))

(fn AllTargetsDestroyed
  (if (Math|Boolean|ANDBoolean (== (Variables|Default|GetGreen%20Array%20Len) 0) (== (Variables|Default|GetPurple%20Array%20Len) 0) (== (Variables|Default|GetWhite%20Array%20Len) 0))
    (bind _foundwidgets (Widget|GetAllWidgetsOfClass "/Game/Blueprints/Tutorial_Managers/Basic/WBP_Basic.WBP_Basic_C" true))
    (for _array_element _foundwidgets
      (bind _aswbp_basic (Utilities|Casting|CastToWBP_Basic _array_element))
      (Default|SetTutorialTextVisibility _aswbp_basic))))