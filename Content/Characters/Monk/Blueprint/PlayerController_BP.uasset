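; Playable Monk 2D flipbook character, despite the PlayerController name, with Enhanced Input for X-axis movement, jumping and punching.
; Punch input jumps the animation instance to a ground or air attack node by falling state, with a DoOnce reset after a flipbook-length-based delay.
; Tick polls each attack flipbook for its hit frame, destroying matching targets inside that attack's hitbox.
; Capsule overlaps destroy step targets.
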(event OnComponentBeginOverlap(CapsuleComponent)
  (params (OverlappedComponent :type Primitive%20Component%20Object%20Reference) (OtherActor :type Actor%20Object%20Reference) (OtherComp :type Primitive%20Component%20Object%20Reference) (OtherBodyIndex :type Integer) (bFromSweep :type Boolean) (SweepResult :type Hit%20Result%20Structure%20%28by%20ref%29))
  (Actor|DestroyActor (Collision|GetOverlappingActors (Variables|Default|GetCapsuleComponent) "/Game/Blueprints/Targets/BP_Step_Target_Child.BP_Step_Target_Child_C" :!class /Script/Engine.PrimitiveComponent)))

(event Custom|Check%20Hitbox
  ;[1 1 1] Function for hitting things with the Punch Hitbox
  (if (== (Class|PaperFlipbookComponent|GetFlipbook (Variables|Default|GetSprite)) "/Game/Characters/Monk/1_atk/Monk_1_atk.Monk_1_atk")
    (if (== (Class|PaperFlipbookComponent|GetPlaybackPositioninFrames (Variables|Default|GetSprite)) 2)
      (for _array_element (Collision|GetOverlappingActors (Variables|Default|GetPunch%20Hitbox) "/Game/Blueprints/Targets/BP_Target.BP_Target_C" :!class /Script/Engine.PrimitiveComponent)
        (if (!= _array_element self)
          (Actor|DestroyActor _array_element))))))

(event Custom|Check%20AirHitbox
  ;[1 1 1] Function for hitting things with the Air attack hitbox
  (if (== (Class|PaperFlipbookComponent|GetFlipbook (Variables|Default|GetSprite)) "/Game/Characters/Monk/air_atk/MonkAirAttack.MonkAirAttack")
    (if (== (Class|PaperFlipbookComponent|GetPlaybackPositioninFrames (Variables|Default|GetSprite)) 3)
      (for _array_element (Collision|GetOverlappingActors (Variables|Default|GetAir%20Hitbox) "/Game/Blueprints/Targets/BP_AirTarget.BP_AirTarget_C" :!class /Script/Engine.PrimitiveComponent)
        (if (!= _array_element self)
          (Actor|DestroyActor _array_element))))))

(event Input|EnhancedActionEvents|EnhancedInputActionMove_IA
  (params (ActionValue :type Float%20%28double-precision%29) (ElapsedSeconds :type Float%20%28double-precision%29) (TriggeredSeconds :type Float%20%28double-precision%29) (InputAction :type Input%20Action%20Object%20Reference :default "/Game/Inputs/Move_IA.Move_IA"))
  ;[1 1 1] Moving
  (:Triggered
    (Pawn|Input|AddMovementInput "1.000000,0.000000,0.000000" ActionValue false)))

(event Input|EnhancedActionEvents|EnhancedInputActionJump_IA
  (params (ActionValue :type Boolean) (ElapsedSeconds :type Float%20%28double-precision%29) (TriggeredSeconds :type Float%20%28double-precision%29) (InputAction :type Input%20Action%20Object%20Reference :default "/Game/Inputs/Jump_IA.Jump_IA"))
  ;[1 1 1] Jumping
  (:Triggered
    (Character|Jump))
  (:Canceled
    (Character|StopJumping)))

(event Input|EnhancedActionEvents|EnhancedInputActionPunch_IA
  (params (ActionValue :type Boolean) (ElapsedSeconds :type Float%20%28double-precision%29) (TriggeredSeconds :type Float%20%28double-precision%29) (InputAction :type Input%20Action%20Object%20Reference :default "/Game/Inputs/Punch_IA.Punch_IA"))
  ;[1 1 1] Attack System
  (:Started
    ;;[1 1 1] Ground Attack
    (Utilities|FlowControl|DoOnce false :!label _label
      (:Completed
        (if (AI|Components|NavMovement|IsFalling (Variables|Character|GetCharacterMovement))
          ;;[1 1 1] Air Attack
          (Class|PaperZDAnimInstance|JumptoNode (Variables|/Script/PaperZD.PaperZDAnimationComponent|GetAnimInstance (Variables|Default|GetAnimationComponent)) "AirAttack" "None")
          (Utilities|FlowControl|Delay (+ (Class|PaperFlipbookComponent|GetFlipbookLength (Variables|Default|GetSprite)) 0.5))
          (goto _label Reset)
          (else
            (Class|PaperZDAnimInstance|JumptoNode (Variables|/Script/PaperZD.PaperZDAnimationComponent|GetAnimInstance (Variables|Default|GetAnimationComponent)) "Attack" "None")
            (Utilities|FlowControl|Delay (- (Class|PaperFlipbookComponent|GetFlipbookLength (Variables|Default|GetSprite)) 0.5))
            (goto _label Reset)))))))

(event EventBeginPlay
  ;[1 1 1] Add mapping context
  (bind _asplayer_controller (Utilities|Casting|CastToPlayerController (Pawn|GetController)))
  (Utilities|IsValid (PlayerController|LocalPlayerSubsystems|GetEnhancedInputLocalPlayerSubsystem _asplayer_controller)
    (:Is%20Valid
      (Input|AddMappingContext (PlayerController|LocalPlayerSubsystems|GetEnhancedInputLocalPlayerSubsystem _asplayer_controller) "/Game/Inputs/Fighting_IMC.Fighting_IMC" 0 "(bIgnoreAllPressedKeysUntilRelease=True,bForceImmediately=False)"))))

(event EventTick
  (params (DeltaSeconds :type Float%20%28single-precision%29))
  (CallFunction|CheckHitbox)
  (CallFunction|CheckAirHitbox))

(fn ConstructionScript)